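; BP_Ammunition_Mashine_Gun is a machine gun ammo pickup that rotates and bobs in place.
; On sphere overlap it checks the actor against all BP_FPS_Player instances, then adds ammo for its weapon ID, plays an equip sound and destroys itself.
; Tick spins the sphere by a configurable yaw speed and starts an UpDown timeline once, which drives the vertical offset with configurable speed and strength.
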(event OnComponentBeginOverlap(Sphere)
  (params (OverlappedComponent :type Primitive%20Component%20Object%20Reference) (OtherActor :type Actor%20Object%20Reference) (OtherComp :type Primitive%20Component%20Object%20Reference) (OtherBodyIndex :type Integer) (bFromSweep :type Boolean) (SweepResult :type Hit%20Result%20Structure%20%28by%20ref%29))
  ;[1 1 1] On Pick Up
  (bind _outactors (Actor|GetAllActorsOfClass "/Game/RetroCore/Blueprints/Player/BP_FPS_Player.BP_FPS_Player_C"))
  (for _array_element _outactors
    (if (== _array_element OtherActor)
      (Default|AddAmmunition _array_element (Variables|Default|GetAmmunition%20to%20Add) (Variables|Default|GetWeapon%20ID))
      (Audio|PlaySoundatLocation "/Game/RetroCore/Audio/SC_AmmoEquip_Mashine_Gun.SC_AmmoEquip_Mashine_Gun" (Transformation|GetActorLocation) "0, 0, 0" 1.0 1.0 0.0 0 0 0 0)
      (Actor|DestroyActor))))

(event EventTick
  (params (DeltaSeconds :type Float%20%28single-precision%29))
  ;[1 1 1] Item Rotation and UpDown Animation
  (Transformation|AddRelativeRotation (Variables|Default|GetSphere) (Math|Rotator|MakeRotator 0.0 0.0 (Variables|Default|GetPickup%20Rotation%20Speed)) false false)
  (Utilities|FlowControl|DoOnce false
    (:Completed
      (Components|Timeline|SetPlayRate (Variables|Default|GetUp%20Down) (Variables|Default|GetPickup%20Up%20Down%20Speed))
      (bind _height (Timeline|Up%20Down Play)
        (:Update
          (Transformation|SetRelativeLocation (Variables|Default|GetSphere) (Math|Vector|MakeVector 0.0 0.0 (* _height (Variables|Default|GetPickup%20Up%20Down%20Strength))) false false))))))

(fn ConstructionScript)