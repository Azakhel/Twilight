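; Floating damage number actor that pops out with a random physics impulse on spawn, scattering sideways and upward.
; SetDamageValue passes the damage, truncated to an integer, to its BP_Damage_Widget widget component for display.
; It also binds the actor's destruction to that widget's destroy callback, so the widget decides when the indicator disappears.
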(event Custom|Set%20Damage%20Value
  (params (Damage%20Value :type Float%20%28double-precision%29))
  (bind _asbp_damage_widget (Utilities|Casting|CastToBP_Damage_Widget (UserInterface|GetUserWidgetObject (Variables|Default|GetWidget))))
  (EventDispatchers|BindEventtoDestroyDamageIndicator _asbp_damage_widget (delegate Custom|Destroy%20Actor))
  (Default|SetDamageValue _asbp_damage_widget (Math|Float|Truncate Damage%20Value)))

(event Custom|Destroy%20Actor
  (Actor|DestroyActor))

(event EventBeginPlay
  (Physics|AddImpulse (Variables|Default|GetPhysics) (Math|Vector|MakeVector (Math|Random|RandomFloatinRange -6e+02 6e+02) (Math|Random|RandomFloatinRange -6e+02 6e+02) (Math|Random|RandomFloatinRange 3e+02 6e+02)) "None" true))

(fn ConstructionScript)