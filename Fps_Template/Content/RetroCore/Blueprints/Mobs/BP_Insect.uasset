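; BP_Insect is a flying enemy that chases the FPS player and damages them on contact with its damage radius.
; FlyingAI homes on the player's capsule, activated while the player is inside the sensing radius and visible to delayed Tick line traces, otherwise deactivated after LastSeenAge.
; AnyDamage optionally spawns damage indicators and reduces health.
; Death enables mesh physics, disables capsule collision, swaps wing audio for a death sound, then destroys the actor after a delay.
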(event OnComponentBeginOverlap(SensingRadius)
  (params (OverlappedComponent :type Primitive%20Component%20Object%20Reference) (OtherActor :type Actor%20Object%20Reference) (OtherComp :type Primitive%20Component%20Object%20Reference) (OtherBodyIndex :type Integer) (bFromSweep :type Boolean) (SweepResult :type Hit%20Result%20Structure%20%28by%20ref%29))
  ;[1 1 1] Player Sensing Radius
  (Utilities|Casting|CastToBP_FPS_Player OtherActor)
  (Variables|Blueprint|SetNear%20Player? true))

(event OnComponentEndOverlap(SensingRadius)
  (params (OverlappedComponent :type Primitive%20Component%20Object%20Reference) (OtherActor :type Actor%20Object%20Reference) (OtherComp :type Primitive%20Component%20Object%20Reference) (OtherBodyIndex :type Integer))
  ;[1 1 1] Player Sensing Radius
  (Utilities|Casting|CastToBP_FPS_Player OtherActor)
  (Variables|Blueprint|SetNear%20Player? false))

(event OnComponentBeginOverlap(DamageRadius)
  (params (OverlappedComponent :type Primitive%20Component%20Object%20Reference) (OtherActor :type Actor%20Object%20Reference) (OtherComp :type Primitive%20Component%20Object%20Reference) (OtherBodyIndex :type Integer) (bFromSweep :type Boolean) (SweepResult :type Hit%20Result%20Structure%20%28by%20ref%29))
  ;[1 1 1] Apply Damage
  (bind _asbp_fps_player (Utilities|Casting|CastToBP_FPS_Player OtherActor))
  (if (not (Variables|Blueprint|GetDead?))
    (Game|Damage|ApplyDamage _asbp_fps_player (Variables|Settings|GetBase%20Damage) 0 self "/Script/Engine.DamageType")))

(event Custom|Chase%20Tick
  ;[1 1 1] Chase Player when Near and in Sight
  (if (and (Variables|Blueprint|GetCan%20See%20Player?) (Variables|Blueprint|GetNear%20Player?))
    (if (not (Variables|Blueprint|GetDead?))
      (Components|Activation|Activate (Variables|Default|GetFlyingAI) false))
    (else
      (Utilities|FlowControl|Delay (Variables|Settings|GetLast%20Seen%20Age))
      (Components|Activation|Deactivate (Variables|Default|GetFlyingAI)))))

(event Custom|Event%20Respawn
  ;[1 1 1] Set Player to Chase
  (Variables|/Script/Engine.ProjectileMovementComponent|SetHomingTargetComponent (Variables|Default|GetFlyingAI) (Variables|/Script/Engine.Character|GetCapsuleComponent (.AsBP%20FPS%20Player (Utilities|Casting|CastToBP_FPS_Player (Game|Player|GetPlayerPawn 0))))))

(event EventBeginPlay
  ;[1 1 1] Set Player to Chase
  (Variables|/Script/Engine.ProjectileMovementComponent|SetHomingTargetComponent (Variables|Default|GetFlyingAI) (Variables|/Script/Engine.Character|GetCapsuleComponent (.AsBP%20FPS%20Player (Utilities|Casting|CastToBP_FPS_Player (Game|Player|GetPlayerPawn 0))))))

(event EventTick
  (params (DeltaSeconds :type Float%20%28single-precision%29))
  ;[1 1 1] Sight Sensing
  (if (Variables|Blueprint|GetDead?)
    (Components|Activation|Deactivate (Variables|Default|GetFlyingAI))
    (else
      (Utilities|FlowControl|Delay (Variables|Settings|GetSight%20Sensing%20Interval))
      (CallFunction|ChaseTick)
      (if (Variables|Blueprint|GetNear%20Player?)
        (bind _outhit (Collision|LineTraceByChannel (Transformation|GetWorldLocation (Variables|Default|GetCapsule)) (Transformation|GetWorldLocation (Variables|/Script/Engine.Character|GetCapsuleComponent (.AsBP%20FPS%20Player (Utilities|Casting|CastToBP_FPS_Player (Game|Player|GetPlayerPawn 0))))) "TraceTypeQuery1" false 0 "None"))
        (if (.bBlockingHit (Collision|BreakHitResult _outhit))
          (Variables|Blueprint|SetCan%20See%20Player? false)
          (else
            (Variables|Blueprint|SetCan%20See%20Player? true)))))))

(event Game|Damage|EventAnyDamage
  (params (Damage :type Float%20%28single-precision%29) (DamageType :type Damage%20Type%20Object%20Reference) (InstigatedBy :type Controller%20Object%20Reference) (DamageCauser :type Actor%20Object%20Reference))
  ;[1 1 1] Receive Damage
  (if (> (Variables|Settings|GetHealth) 0.0)
    (if (Variables|Settings|GetShow%20Damage%20Indicator)
      (bind _returnvalue (Game|SpawnActorfromClass "/Game/RetroCore/Blueprints/Mobs/BP_Damage_Indicator.BP_Damage_Indicator_C" (Math|Transform|MakeTransform (+ (Transformation|GetActorLocation) (Math|Vector|MakeVector 0.0 0.0 (Math|Random|RandomFloatinRange 0.0 1.2e+02))) "0, 0, 0" "1.000000,1.000000,1.000000") "Undefined" "MultiplyWithRoot" 0 0))
      (Default|SetDamageValue _returnvalue Damage))
    (if (> (- (Variables|Settings|GetHealth) Damage) 0.0)
      (Variables|Settings|SetHealth (- (Variables|Settings|GetHealth) Damage))
      (else
        ;[1 1 1] Death
        (Variables|Settings|SetHealth 0.0)
        (Physics|SetSimulatePhysics (Variables|Default|GetMesh) true)
        (Collision|SetCollisionEnabled (Variables|Default|GetCapsule) "NoCollision")
        (Components|Activation|Deactivate (Variables|Default|GetAudio%20Wing%20Flapping))
        (Audio|PlaySoundatLocation "/Game/RetroCore/Audio/SC_Insect_Death.SC_Insect_Death" (Transformation|GetWorldLocation (Variables|Default|GetMesh)) "0, 0, 0" 1.0 1.0 0.0 0 0 0 0)
        (Variables|Blueprint|SetDead? true)
        (Utilities|FlowControl|Delay 1e+01)
        (Actor|DestroyActor)))))

(fn ConstructionScript)