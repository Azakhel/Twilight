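; Melee monster enemy that chases the FPS player when seen or damaged, attacking through a montage whose notify applies sphere-overlap damage.
; Pawn sensing drives AI MoveTo, with retriggerable delays ending the chase after sight is lost.
; Tick uses latent delays to pace idle look-around, drips, idle sounds and screams.
; Damage can spawn floating indicators; death ragdolls the mesh, stops drip effects and destroys the actor after a delay.
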(event OnSeePawn(PawnSensing)
  (params (Pawn :type Pawn%20Object%20Reference))
  ;[1 1 1] On See Pawn
  (if (not (Variables|Blueprint|GetDead?))
    (bind _asbp_fps_player (Utilities|Casting|CastToBP_FPS_Player Pawn))
    (Variables|Blueprint|SetPlayer%20to%20Chase _asbp_fps_player)
    (Variables|Blueprint|SetIdle? false)
    (Utilities|FlowControl|Sequence
      (:then_0
        (Variables|Blueprint|SetCan%20See%20Enemy? true)
        (CallFunction|ChasePlayer (Variables|Blueprint|GetPlayer%20to%20Chase))
        (Utilities|FlowControl|DoOnce false
          (:Completed
            (Audio|Components|Audio|Play (Variables|Default|GetAudio_Scream) 0.0))))
      (:then_1
        (Utilities|FlowControl|RetriggerableDelay 0.2)
        (Variables|Blueprint|SetCan%20See%20Enemy? false)))))

(event Custom|Chase%20Player
  (params (Player%20to%20Chase :type Pawn%20Object%20Reference))
  ;[1 1 1] Chase Player
  (AI|AIMoveTo self "0, 0, 0" Player%20to%20Chase 1.8e+02 false
    (:OnSuccess
      ;[1 1 1] Attack
      (if (and (Variables|Blueprint|GetCan%20Attack?) (not (Variables|Blueprint|GetDead?)))
        (Variables|Blueprint|SetCan%20Attack? false)
        (Animation|Montage|PlayMontage (Variables|Character|GetMesh) "/Game/RetroCore/Animation/AM_Monster_Attack.AM_Monster_Attack"
          (:OnCompleted
            (Variables|Blueprint|SetCan%20Attack? true)
            (CallFunction|ChasePlayer (Variables|Blueprint|GetPlayer%20to%20Chase)))
          (:OnNotifyBegin
            (if (Audio|Components|Audio|IsPlaying (Variables|Default|GetAudio_Scream))
              _
              (else
                (Audio|Components|Audio|Play (Variables|Default|GetAudio_Scream) 0.0)))
            (bind _outactors (Collision|SphereOverlapActors (Transformation|GetWorldLocation (Variables|Default|GetSphere_Damage)) 1.7e+02 (Utilities|Array|MakeArray "ObjectTypeQuery3") "/Game/RetroCore/Blueprints/Player/BP_FPS_Player.BP_FPS_Player_C" (Utilities|Array|MakeArray self)))
            (for _array_element _outactors
              (Game|Damage|ApplyDamage _array_element (Variables|Settings|GetBase%20Damage) (Pawn|GetController) self "/Script/Engine.DamageType"))))))))

(event Custom|Stop%20Chase
  ;[1 1 1] Stop Chase
  (Variables|Blueprint|SetIdle? true)
  (AI|Navigation|StopMovement (AI|GetAIController self))
  ;[1 1 1] On See Pawn
  (Utilities|FlowControl|DoOnce false) ; enters at Reset
)

(event Custom|Drip
  ;[1 1 1] Drip/Idle/Scream Sound
  (Utilities|FlowControl|Delay (Math|Random|RandomFloatinRange 0.1 1.2))
  (Audio|Components|Audio|Play (Variables|Default|GetAudio_Drip) 0.0))

(event Custom|Idle
  ;[1 1 1] Drip/Idle/Scream Sound
  (Utilities|FlowControl|Delay (Math|Random|RandomFloatinRange 8.0 14.0))
  (if (not (Variables|Blueprint|GetDead?))
    (Audio|Components|Audio|Play (Variables|Default|GetAudio_Idle) 0.0)))

(event Custom|Scream%20while%20Chasing
  ;[1 1 1] Drip/Idle/Scream Sound
  (Utilities|FlowControl|Delay (Math|Random|RandomFloatinRange 3.0 6.0))
  (if (Math|Boolean|ANDBoolean (Variables|Blueprint|GetCan%20See%20Enemy?) (Variables|Blueprint|GetCan%20Attack?) (not (Variables|Blueprint|GetDead?)))
    (Audio|Components|Audio|Play (Variables|Default|GetAudio_Scream) 0.0)))

(event Custom|Is%20Hit
  ;[1 1 1] Chase Player when Hit
  (CallFunction|ChasePlayer))

(event Custom|Idle%20Look
  ;[1 1 1] Idle Looking Around
  (if (and (Variables|Blueprint|GetIdle?) (Variables|Settings|GetShould%20Look%20Around%20if%20Idle))
    (Utilities|FlowControl|Sequence
      (:then_0
        (Utilities|FlowControl|Delay (Math|Random|RandomFloatinRange 1.0 3.0))
        (Variables|Blueprint|SetIdle%20Look%20At (Math|Random|RandomFloatinRange 0.0 3.6e+02)))
      (:then_1
        (Transformation|SetActorRotation (Math|Rotator|MakeRotator 0.0 0.0 (.yaw (Class|KismetMathLibrary|RInterptoConstant (Transformation|GetActorRotation) (Math|Rotator|MakeRotator 0.0 0.0 (Variables|Blueprint|GetIdle%20Look%20At)) (Utilities|Time|GetWorldDeltaSeconds) 1e+01))))))))

(event EventTick
  (params (DeltaSeconds :type Float%20%28single-precision%29))
  ;[1 1 1] Stop Chasing after set Time
  (if (not (Variables|Blueprint|GetDead?))
    (CallFunction|IdleLook)
    ;;[1 1 1] Audio
    (CallFunction|Idle)
    (CallFunction|Drip)
    (CallFunction|ScreamWhileChasing)
    (if (Variables|Blueprint|GetCan%20See%20Enemy?)
      ;;[1 1 1] Chase Duration after Enemy no longer can see the Player
      (Utilities|FlowControl|RetriggerableDelay (Variables|Settings|GetLast%20Seen%20Age))
      (if (not (Variables|Blueprint|GetCan%20See%20Enemy?))
        (CallFunction|StopChase)))))

(event Game|Damage|EventAnyDamage
  (params (Damage :type Float%20%28single-precision%29) (DamageType :type Damage%20Type%20Object%20Reference) (InstigatedBy :type Controller%20Object%20Reference) (DamageCauser :type Actor%20Object%20Reference))
  (bind _mesh (Variables|Character|GetMesh))
  ;[1 1 1] Receive Damage
  (if (Variables|Blueprint|GetIdle?)
    (CallFunction|ChasePlayer (.AsBP%20FPS%20Player (Utilities|Casting|CastToBP_FPS_Player (Game|Player|GetPlayerPawn 0)))))
  (if (> (Variables|Settings|GetHealth) 0.0)
    (if (Variables|Settings|GetShow%20Damage%20Indicator)
      (bind _returnvalue (Game|SpawnActorfromClass "/Game/RetroCore/Blueprints/Mobs/BP_Damage_Indicator.BP_Damage_Indicator_C" (Math|Transform|MakeTransform (+ (Transformation|GetActorLocation) (Math|Vector|MakeVector 0.0 0.0 (Math|Random|RandomFloatinRange 0.0 1.2e+02))) "0, 0, 0" "1.000000,1.000000,1.000000") "Undefined" "MultiplyWithRoot" 0 0))
      (Default|SetDamageValue _returnvalue Damage))
    (if (> (- (Variables|Settings|GetHealth) Damage) 0.0)
      (Variables|Settings|SetHealth (- (Variables|Settings|GetHealth) Damage))
      (else
        ;[1 1 1] Death
        (Variables|Settings|SetHealth 0.0)
        (Physics|SetSimulatePhysics _mesh true)
        (Physics|AddImpulse _mesh (* (Math|Vector|GetForwardVector _mesh) -2.5e+04) "None" false)
        (Pawn|Components|CharacterMovement|DisableMovement (Variables|Character|GetCharacterMovement))
        (Niagara|SetNiagaraVariable(Float) (Variables|Default|GetNS_Drip5) "SpawnRate" 0.0)
        (Variables|Blueprint|SetDead? true)
        (Audio|Components|Audio|Stop (Variables|Default|GetAudio_Liquid))
        (Collision|SetCollisionEnabled (Variables|Collision|GetCapsuleComponent) "NoCollision")
        (Audio|PlaySoundatLocation "/Game/RetroCore/Audio/SC_Monster_Death.SC_Monster_Death" (Transformation|GetWorldLocation (Variables|Character|GetMesh)) "0, 0, 0" 1.0 1.0 0.0 0 0 0 0)
        (Utilities|FlowControl|Delay 1e+01)
        (Actor|DestroyActor)))))

(fn ConstructionScript)