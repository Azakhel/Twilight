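; BP_Explosion is a reusable explosion helper for weapons that acts at the location of its owning actor, cached on BeginPlay.
; Initialize stores an optional radial force component supplied by the caller.
; Explode plays the explosion sound, fires that component's impulse if valid, then applies radial damage with caller-supplied damage and radius, using the Pawn channel for damage prevention.
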(event EventBeginPlay
  (Variables|Default|SetOwner (Components|GetOwner)))

(event EventTick
  (params (DeltaSeconds :type Float%20%28single-precision%29)))

(fn Explode
  (params (Damage :type Float%20%28single-precision%29) (Damage%20Radius :type Float%20%28single-precision%29))
  (Audio|PlaySoundatLocation "/Game/RetroCore/Audio/SC_Explosion.SC_Explosion" (Transformation|GetActorLocation (Variables|Default|GetOwner)) "0, 0, 0" 1.0 1.0 0.0 0 0 0 0)
  (Utilities|FlowControl|Sequence
    (:then_0
      (Utilities|IsValid (Variables|Default|GetRadial%20Force%20Component)
        (:Is%20Valid
          (Class|RadialForceComponent|FireImpulse (Variables|Default|GetRadial%20Force%20Component)))))
    (:then_1
      (Game|Damage|ApplyRadialDamage Damage (Transformation|GetActorLocation (Variables|Default|GetOwner)) Damage%20Radius 0 0 (Variables|Default|GetOwner) 0 false "ECC_Pawn"))))

(fn Initialize
  (params (Radial%20Force%20Component :type Radial%20Force%20Component%20Object%20Reference))
  (Variables|Default|SetRadial%20Force%20Component Radial%20Force%20Component))