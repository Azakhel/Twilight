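; Laser weapon for the FPS player that doubles as its own spinning, bobbing world pickup.
; Shortly after BeginPlay it either arms or enables pickup; overlap gives new owners the weapon class and ammo, then destroys the actor.
; Fire line-traces from the camera, damaging only "enemy" or "destructable" tagged actors, with cooldown via DoOnce and Delay.
; Niagara beam, impact and flash effects accompany timeline-driven recoil, barrel rotation and muzzle light.
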(event OnComponentBeginOverlap(Sphere)
  (params (OverlappedComponent :type Primitive%20Component%20Object%20Reference) (OtherActor :type Actor%20Object%20Reference) (OtherComp :type Primitive%20Component%20Object%20Reference) (OtherBodyIndex :type Integer) (bFromSweep :type Boolean) (SweepResult :type Hit%20Result%20Structure%20%28by%20ref%29))
  ;[1 1 1] Pick Up On Overlap
  (Utilities|FlowControl|Gate true
    (:Exit
      (bind _outactors (Actor|GetAllActorsOfClass "/Game/RetroCore/Blueprints/Player/BP_FPS_Player.BP_FPS_Player_C"))
      (for _array_element _outactors
        (if (== _array_element OtherActor)
          (Variables|Blueprint|SetOverlappingPlayer _array_element)
          (Variables|Blueprint|SetFoundPlayer true)
          (if (.ReturnValue (Utilities|Map|Find (Variables|/Game/RetroCore/Blueprints/Player/BP_FPS_Player.BP_FPS_Player_C|GetWeapon%20Inventory%20Class _array_element) (Variables|Settings|GetWeapon%20ID)))
            (Variables|Blueprint|SetIsAlreadyPickedUp? true))))
      (if (Variables|Blueprint|GetFoundPlayer)
        (if (not (Variables|Blueprint|GetIsAlreadyPickedUp?))
          (Default|PickedUpNewWeapon (Variables|Blueprint|GetOverlappingPlayer) (Variables|Settings|GetWeapon%20ID) (Utilities|GetClass self) (Variables|Settings|GetStarting%20Ammunition))
          (Actor|DestroyActor))))))

(event Custom|Rotate
  ;[1 1 1] Item Rotation and UpDown Animation (as a PickUp)
  (Transformation|SetRelativeScale3D (Variables|Default|GetDefaultSceneRoot) "1.600000,1.600000,1.600000")
  (Utilities|FlowControl|Gate true) ; enters at Open
)

(event Custom|Fire
  (bind _sphere (Variables|Default|GetSphere))
  (bind _playerusingthisweapon (Variables|Blueprint|GetPlayerUsingThisWeapon))
  (bind _pointlight (Variables|Default|GetPointLight))
  (bind _weapon_range (Variables|Settings|GetWeapon%20Range))
  (bind _playerusingthisweapon_2 (Variables|Blueprint|GetPlayerUsingThisWeapon))
  (bind _playerusingthisweapon_3 (Variables|Blueprint|GetPlayerUsingThisWeapon))
  (bind _empty_actor (Variables|Blueprint|GetEmpty%20Actor))
  (bind _returnvalue (Transformation|GetWorldLocation _sphere))
  (bind _camera (Variables|/Game/RetroCore/Blueprints/Player/BP_FPS_Player.BP_FPS_Player_C|GetCamera _playerusingthisweapon))
  (bind _camera_2 (Variables|/Game/RetroCore/Blueprints/Player/BP_FPS_Player.BP_FPS_Player_C|GetCamera _playerusingthisweapon_2))
  (bind _camera_3 (Variables|/Game/RetroCore/Blueprints/Player/BP_FPS_Player.BP_FPS_Player_C|GetCamera _playerusingthisweapon_3))
  (bind _returnvalue_2 (Math|Vector|GetForwardVector _camera_3))
  (bind _returnvalue_3 (Transformation|GetWorldLocation _camera_2))
  (bind _returnvalue_4 (Transformation|GetWorldLocation _camera))
  (bind _returnvalue_5 (* _returnvalue_2 _weapon_range))
  (bind _returnvalue_6 (- _returnvalue_4 _returnvalue))
  (bind _returnvalue_7 (+ _returnvalue_6 _returnvalue_5))
  ;[1 1 1] Fire Weapon
  (if (Variables|Blueprint|GetArmed)
    (Utilities|FlowControl|Sequence
      (:then_0
        (Utilities|FlowControl|DoOnce false :!label _label
          (:Completed
            (Default|SubtractAmmunition (Variables|Blueprint|GetPlayerUsingThisWeapon))
            (Audio|PlaySoundatLocation "/Game/RetroCore/Audio/SC_Laser_Shot.SC_Laser_Shot" (Transformation|GetWorldLocation (Variables|Default|GetPointLight)) "0, 0, 0" 1.0 1.0 0.0 0 0 0 0)
            ;;[1 1 1] Line Trace and Laser Niagara Effect
            (bind _outhit (Collision|LineTraceByChannel _returnvalue_3 (+ _returnvalue_3 (* (Math|Vector|GetForwardVector _camera_2) (Variables|Settings|GetWeapon%20Range))) "TraceTypeQuery2" false (Utilities|Array|MakeArray (Variables|Blueprint|GetPlayerUsingThisWeapon)) "None"))
            (bind _returnvalue_8 (Niagara|SpawnSystematLocation "/Game/RetroCore/Niagara/NS_Laser.NS_Laser" (Transformation|GetWorldLocation (Variables|Default|GetPointLight))))
            (Effects|Components|ParticleSystem|SetColorParameter _returnvalue_8 "Beam Color" (Variables|Settings|GetBeam%20Color))
            (if (.bBlockingHit (Collision|BreakHitResult _outhit))
              (if (Actor|ActorHasTag (.HitActor (Collision|BreakHitResult _outhit)) "enemy")
                (Variables|Default|SetNiagara%20Hit%20Effect "/Game/RetroCore/Niagara/NS_Blood.NS_Blood")
                (Variables|Blueprint|SetHit%20Actor (.HitActor (Collision|BreakHitResult _outhit)) :!label _label_2)
                (Niagara|SpawnSystematLocation (Variables|Default|GetNiagara%20Hit%20Effect) (.Location (Collision|BreakHitResult _outhit)))
                (elif (Actor|ActorHasTag (.HitActor (Collision|BreakHitResult _outhit)) "destructable")
                  (Variables|Default|SetNiagara%20Hit%20Effect "/Game/RetroCore/Niagara/NS_Wood_Chipping.NS_Wood_Chipping")
                  (goto _label_2)
                  (else
                    (Variables|Blueprint|SetHit%20Actor _empty_actor))))
              (Effects|Components|ParticleSystem|SetVectorParameter _returnvalue_8 "Beam End" (+ _returnvalue_6 (* _returnvalue_2 (.Distance (Collision|BreakHitResult _outhit)))))
              (Effects|Components|ParticleSystem|SetVectorParameter _returnvalue_8 "Beam Shell Scale" (Math|Vector|MakeVector (Math|Vector|VectorLength (+ _returnvalue_6 (* _returnvalue_2 (.Distance (Collision|BreakHitResult _outhit))))) 1e+01 1e+01))
              (if (== (Variables|Blueprint|GetHit%20Actor) (Variables|Blueprint|GetEmpty%20Actor))
                (bind _returnvalue_9 (Niagara|SpawnSystematLocation "/Game/RetroCore/Niagara/NS_Beam_Impact.NS_Beam_Impact" (+ (.Location (Collision|BreakHitResult _outhit)) (Math|Vector|Normalize (.ImpactNormal (Collision|BreakHitResult _outhit))))))
                (Effects|Components|ParticleSystem|SetVectorParameter _returnvalue_9 "Impact Normal" (Math|Vector|MakeVector (.X (Math|Vector|BreakVector (.ImpactNormal (Collision|BreakHitResult _outhit)))) (.Y (Math|Vector|BreakVector (.ImpactNormal (Collision|BreakHitResult _outhit)))) (.Z (Math|Vector|BreakVector (.ImpactNormal (Collision|BreakHitResult _outhit))))))
                (Effects|Components|ParticleSystem|SetColorParameter _returnvalue_9 "Impact Color" (Variables|Settings|GetBeam%20Color)))
              (else
                (Variables|Blueprint|SetHit%20Actor _empty_actor)
                (Effects|Components|ParticleSystem|SetVectorParameter _returnvalue_8 "Beam End" _returnvalue_7)
                (Effects|Components|ParticleSystem|SetVectorParameter _returnvalue_8 "Beam Shell Scale" (Math|Vector|MakeVector (Math|Vector|VectorLength _returnvalue_7) 1e+01 1e+01))))
            ;;[1 1 1] Damage
            (Game|Damage|ApplyDamage (Variables|Blueprint|GetHit%20Actor) (* (Variables|Settings|GetBase%20Damage) (Variables|/Game/RetroCore/Blueprints/Player/BP_FPS_Player.BP_FPS_Player_C|GetDamage%20Multiplier (Variables|Blueprint|GetPlayerUsingThisWeapon))) 0 self)
            ;;[1 1 1] Muzzle Flash
            (Rendering|Components|Light|SetLightColor _pointlight (Variables|Settings|GetBeam%20Color) true)
            (bind _returnvalue_10 (Niagara|SpawnSystemAttached "/Game/RetroCore/Niagara/NS_Beam_Flash.NS_Beam_Flash" _pointlight "None" "0, 0, 0" "0, 0, 0" "KeepRelativeOffset" false))
            (bind _returnvalue_11 (Rendering|Material|CreateDynamicMaterialInstance "/Game/RetroCore/Materials/Niagara/M_Beam_Flash.M_Beam_Flash" "None" "None" :!class /Script/Engine.KismetMaterialLibrary))
            (Class|NiagaraComponent|SetVariableMaterial _returnvalue_10 "Dynamic Flash" _returnvalue_11)
            (Effects|Components|ParticleSystem|SetColorParameter _returnvalue_10 "Flash Color" (Variables|Settings|GetBeam%20Color))
            ;;[1 1 1] Kickback & Light Animation
            (Variables|Blueprint|SetRandom%20Pitch (Math|Random|RandomFloatinRange -0.2 0.2))
            (Variables|Blueprint|SetRandom%20Yaw (Math|Random|RandomFloatinRange -0.4 0.4))
            (bind (_direction _kickback _light _barrel_rotation) (Timeline|Fire%20Animation PlayFromStart)
              (:Update
                (Rendering|Components|Light|SetIntensity (Variables|Default|GetPointLight) (* _light 3e+03))
                (Transformation|SetRelativeRotation (Variables|Default|GetSM_Laser_Barrel) (Math|Rotator|MakeRotator (* _barrel_rotation -1e+01) 0.0 0.0) false false)
                (Transformation|SetRelativeLocation (Variables|Default|GetSM_Laser_Body) (Math|Vector|MakeVector (* (* _kickback -1.0) 0.85) 0.0 0.0) false false)
                (Transformation|SetRelativeRotation (Variables|Default|GetSM_Laser_Body) (Math|Rotator|MakeRotator 0.0 (* (* _kickback -1.0) (Variables|Blueprint|GetRandom%20Pitch)) (* (* _kickback -1.0) (Variables|Blueprint|GetRandom%20Yaw))) false false))))))
      (:then_1
        (Utilities|FlowControl|Delay (Variables|Settings|GetWeapon%20Cooldown%20Duration))
        (goto _label Reset)))))

(event EventTick
  (params (DeltaSeconds :type Float%20%28single-precision%29))
  ;[1 1 1] Item Rotation and UpDown Animation (as a PickUp)
  (Utilities|FlowControl|Gate true
    (:Exit
      (Transformation|AddRelativeRotation (Variables|Default|GetSM_Laser_Body) (Math|Rotator|MakeRotator 0.0 0.0 (Variables|Settings|GetPickup%20Rotation%20Speed)) false false)
      (Utilities|FlowControl|DoOnce false
        (:Completed
          (Components|Timeline|SetPlayRate (Variables|Default|GetUpDown) (Variables|Settings|GetPickupUpDown%20Speed))
          (bind _height (Timeline|UpDown Play)
            (:Update
              (Transformation|SetRelativeLocation (Variables|Default|GetSM_Laser_Body) (Math|Vector|MakeVector 0.0 0.0 (* _height (Variables|Settings|GetPickup%20UpDown%20Strength))) false false))))))))

(event EventBeginPlay
  ;[1 1 1] Enable Overlap if not Picked Up
  (Utilities|FlowControl|Delay 0.1)
  (if (Variables|Blueprint|GetIsPickedUp?)
    (Variables|Blueprint|SetArmed true)
    (else
      ;[1 1 1] Pick Up On Overlap
      (CallFunction|Rotate)
      (Utilities|FlowControl|Gate true) ; enters at Open
    )))

(fn ConstructionScript)