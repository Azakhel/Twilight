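; BP_Rocket is a weapon projectile that explodes on hitting anything other than the player who fired it, or after a ten-second fuse.
; Both triggers share one detonation path, with DoOnce guarding only repeated hits.
; BPExplosion deals radial damage scaled by the player's damage multiplier, and a sprite explosion actor spawns.
; Sound, exhaust, mesh and light are shut off before delayed destruction.
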(event Collision|EventHit
  (params (MyComp :type Primitive%20Component%20Object%20Reference) (Other :type Actor%20Object%20Reference) (OtherComp :type Primitive%20Component%20Object%20Reference) (bSelfMoved :type Boolean) (HitLocation :type Vector :default "0, 0, 0") (HitNormal :type Vector :default "0, 0, 0") (NormalImpulse :type Vector :default "0, 0, 0") (Hit :type Hit%20Result%20Structure%20%28by%20ref%29))
  (if (not (== Other (Variables|Default|GetPlayerUsingThisWeapon)))
    (Utilities|FlowControl|DoOnce false
      (:Completed
        (Default|Explode (Variables|Default|GetBP_Explosion) (* (Variables|/Game/RetroCore/Blueprints/Player/BP_FPS_Player.BP_FPS_Player_C|GetDamage%20Multiplier (Variables|Default|GetPlayerUsingThisWeapon)) (Variables|Default|GetBase%20Damage)) (Variables|Default|GetDamage%20Radius))
        (Audio|Components|Audio|Stop (Variables|Default|GetSC_Rocket))
        (bind _returnvalue (Game|SpawnActorfromClass "/Game/RetroCore/Blueprints/Weapons/BP_Sprite_Explosion.BP_Sprite_Explosion_C" (Math|Transform|MakeTransform (Transformation|GetWorldLocation (Variables|Default|GetSpriteSpawnLoc)) "0, 0, 0" "1.000000,1.000000,1.000000") "AlwaysSpawn" "MultiplyWithRoot" 0 0))
        (Variables|/Game/RetroCore/Blueprints/Weapons/BP_Sprite_Explosion.BP_Sprite_Explosion_C|SetPlayer%20Reference _returnvalue (Variables|Default|GetPlayerUsingThisWeapon))
        (Components|Activation|Deactivate (Variables|Default|GetNS_Rocket_Exhaust))
        (Rendering|SetVisibility (Variables|Default|GetSM_Rocket) false false)
        (Rendering|Components|Light|SetIntensity (Variables|Default|GetPointLight) 0.0)
        (Utilities|FlowControl|Delay 3.0)
        (Actor|DestroyActor)))))

(event EventBeginPlay
  (Default|Initialize (Variables|Default|GetBP_Explosion) (Variables|Default|GetRadialForce))
  (Utilities|FlowControl|Delay 1e+01)
  (Default|Explode (Variables|Default|GetBP_Explosion) (* (Variables|/Game/RetroCore/Blueprints/Player/BP_FPS_Player.BP_FPS_Player_C|GetDamage%20Multiplier (Variables|Default|GetPlayerUsingThisWeapon)) (Variables|Default|GetBase%20Damage)) (Variables|Default|GetDamage%20Radius))
  (Audio|Components|Audio|Stop (Variables|Default|GetSC_Rocket))
  (bind _returnvalue (Game|SpawnActorfromClass "/Game/RetroCore/Blueprints/Weapons/BP_Sprite_Explosion.BP_Sprite_Explosion_C" (Math|Transform|MakeTransform (Transformation|GetWorldLocation (Variables|Default|GetSpriteSpawnLoc)) "0, 0, 0" "1.000000,1.000000,1.000000") "AlwaysSpawn" "MultiplyWithRoot" 0 0))
  (Variables|/Game/RetroCore/Blueprints/Weapons/BP_Sprite_Explosion.BP_Sprite_Explosion_C|SetPlayer%20Reference _returnvalue (Variables|Default|GetPlayerUsingThisWeapon))
  (Components|Activation|Deactivate (Variables|Default|GetNS_Rocket_Exhaust))
  (Rendering|SetVisibility (Variables|Default|GetSM_Rocket) false false)
  (Rendering|Components|Light|SetIntensity (Variables|Default|GetPointLight) 0.0)
  (Utilities|FlowControl|Delay 3.0)
  (Actor|DestroyActor))

(fn ConstructionScript)