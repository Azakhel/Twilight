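; BP_Weapon_Template is a template FPS weapon that serves as both a rotating, bobbing world pickup and the held hitscan gun.
; BeginPlay either arms it or opens gates for pickup animation and overlap, which grants unowned weapons to the player.
; Fire is cooldown-limited, spending ammo, playing audio and randomized muzzle flash, then tracing from the camera.
; Actor tags select blood, wood or wall impact effects and whether damage, scaled by player multiplier, lands.
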(event OnComponentBeginOverlap(PickupCollider)
  (params (OverlappedComponent :type Primitive%20Component%20Object%20Reference) (OtherActor :type Actor%20Object%20Reference) (OtherComp :type Primitive%20Component%20Object%20Reference) (OtherBodyIndex :type Integer) (bFromSweep :type Boolean) (SweepResult :type Hit%20Result%20Structure%20%28by%20ref%29))
  ;[0 0 0] Pickup Item Code
  ;;[1 1 1] Pick Up On Overlap
  (Utilities|FlowControl|Gate true
    (:Exit
      (bind _outactors (Actor|GetAllActorsOfClass "/Game/RetroCore/Blueprints/Player/BP_FPS_Player.BP_FPS_Player_C"))
      (for _array_element _outactors
        (if (== _array_element OtherActor)
          (Variables|Blueprint|SetOverlappingPlayer _array_element)
          (Variables|Blueprint|SetFoundPlayer true)
          (if (.ReturnValue (Utilities|Map|Find (Variables|/Game/RetroCore/Blueprints/Player/BP_FPS_Player.BP_FPS_Player_C|GetWeapon%20Inventory%20Class _array_element) (Variables|Settings|GetWeapon%20ID)))
            (Variables|Blueprint|SetIsAlreadyPickedUp? true))))
      (if (Variables|Blueprint|GetFoundPlayer)
        (if (not (Variables|Blueprint|GetIsAlreadyPickedUp?))
          (Default|PickedUpNewWeapon (Variables|Blueprint|GetOverlappingPlayer) (Variables|Settings|GetWeapon%20ID) (Utilities|GetClass self) (Variables|Settings|GetStarting%20Ammunition))
          (Actor|DestroyActor))))))

(event Custom|Rotate
  ;[0 0 0] Pickup Item Code
  ;;[1 1 1] Item Rotation and UpDown Animation
  (Transformation|SetRelativeScale3D (Variables|Default|GetDefaultSceneRoot) "1.600000,1.600000,1.600000")
  (Utilities|FlowControl|Gate true) ; enters at Open
)

(event Custom|Fire
  (bind _playerusingthisweapon (Variables|Blueprint|GetPlayerUsingThisWeapon))
  (bind _empty_actor (Variables|Blueprint|GetEmpty%20Actor))
  (bind _camera (Variables|/Game/RetroCore/Blueprints/Player/BP_FPS_Player.BP_FPS_Player_C|GetCamera _playerusingthisweapon))
  (bind _returnvalue (Transformation|GetWorldLocation _camera))
  ;[1 1 1] Shoot Weapon, Subtract Ammunition and Play Shoot Audio
  (if (Variables|Blueprint|GetArmed)
    (Utilities|FlowControl|Sequence
      (:then_0
        (Utilities|FlowControl|DoOnce false :!label _label
          (:Completed
            (Default|SubtractAmmunition (Variables|Blueprint|GetPlayerUsingThisWeapon))
            (Audio|PlaySoundatLocation (Variables|Settings|GetShoot%20Audio) (Transformation|GetWorldLocation (Variables|Default|GetMuzzleFlash)) "0, 0, 0" 1.0 1.0 0.0 0 0 0 0)
            ;[0.5782 1 0.5986] Modify this Code to your likings
            ;;[1 1 1] Muzzle Flash
            (bind _returnvalue_2 (Niagara|SpawnSystemAttached "/Game/RetroCore/Niagara/NS_Muzzle_Flash.NS_Muzzle_Flash" (Variables|Default|GetMuzzleFlash) "None" "0, 0, 0" "0, 0, 0" "KeepRelativeOffset" false))
            (bind _returnvalue_3 (Rendering|Material|CreateDynamicMaterialInstance "/Game/RetroCore/Materials/Niagara/M_Muzzle_Flash.M_Muzzle_Flash" "None" "None" :!class /Script/Engine.KismetMaterialLibrary))
            (Rendering|Material|SetTextureParameterValue _returnvalue_3 "Flash Texture" (Utilities|Array|Get(acopy) (Variables|Blueprint|GetMuzzleFlashes) (Math|Random|RandomIntegerinRange 0 7)))
            (Class|NiagaraComponent|SetVariableMaterial _returnvalue_2 "Dynamic Flash" _returnvalue_3)
            (Effects|Components|ParticleSystem|SetColorParameter _returnvalue_2 "Flash Color" "(R=5.000000,G=2.735661,B=0.497275,A=1.000000)")
            (Utilities|FlowControl|Sequence
              (:then_0
                ;;[1 1 1] Line Trace
                (bind _outhit (Collision|LineTraceByChannel _returnvalue (+ _returnvalue (* (Math|Vector|GetForwardVector _camera) (Variables|Settings|GetWeapon%20Range))) "TraceTypeQuery2" false (Utilities|Array|MakeArray (Variables|Blueprint|GetPlayerUsingThisWeapon)) "None"))
                ;;[1 1 1] Hit Result
                (if (.bBlockingHit (Collision|BreakHitResult _outhit))
                  (if (Actor|ActorHasTag (.HitActor (Collision|BreakHitResult _outhit)) "enemy")
                    (Variables|Default|SetNiagara%20Hit%20Effect "/Game/RetroCore/Niagara/NS_Blood.NS_Blood")
                    (Variables|Blueprint|SetHit%20Actor (.HitActor (Collision|BreakHitResult _outhit)) :!label _label_2)
                    ;;;[1 1 1] Spawn Blood/Chippings Effect when hitting Enemy/Destructable
                    (Niagara|SpawnSystematLocation (Variables|Default|GetNiagara%20Hit%20Effect) (.Location (Collision|BreakHitResult _outhit)))
                    (elif (Actor|ActorHasTag (.HitActor (Collision|BreakHitResult _outhit)) "destructable")
                      (Variables|Default|SetNiagara%20Hit%20Effect "/Game/RetroCore/Niagara/NS_Wood_Chipping.NS_Wood_Chipping")
                      (goto _label_2)
                      (else
                        (Variables|Blueprint|SetHit%20Actor _empty_actor))))
                  (if (== (Variables|Blueprint|GetHit%20Actor) (Variables|Blueprint|GetEmpty%20Actor))
                    ;;;[1 1 1] Spanw Impact Effect when hitting Wall, etc.
                    (bind _returnvalue_4 (Niagara|SpawnSystematLocation "/Game/RetroCore/Niagara/NS_Pellet_Impact.NS_Pellet_Impact" (+ (.Location (Collision|BreakHitResult _outhit)) (Math|Vector|Normalize (.ImpactNormal (Collision|BreakHitResult _outhit))))))
                    (Effects|Components|ParticleSystem|SetVectorParameter _returnvalue_4 "Impact Normal" (Math|Vector|MakeVector (.X (Math|Vector|BreakVector (.ImpactNormal (Collision|BreakHitResult _outhit)))) (.Y (Math|Vector|BreakVector (.ImpactNormal (Collision|BreakHitResult _outhit)))) (.Z (Math|Vector|BreakVector (.ImpactNormal (Collision|BreakHitResult _outhit)))))))
                  (else
                    (Variables|Blueprint|SetHit%20Actor _empty_actor)))
                ;;[1 1 1] Apply Damage
                (Game|Damage|ApplyDamage (Variables|Blueprint|GetHit%20Actor) (* (Variables|Settings|GetBase%20Damage) (Variables|/Game/RetroCore/Blueprints/Player/BP_FPS_Player.BP_FPS_Player_C|GetDamage%20Multiplier (Variables|Blueprint|GetPlayerUsingThisWeapon))) 0 self))
              (:then_1
                (bind _light (Timeline|Animation PlayFromStart)
                  (:Update
                    (Rendering|Components|Light|SetIntensity (Variables|Default|GetMuzzleFlash) (* _light 3e+03)))))))))
      (:then_1
        (Utilities|FlowControl|Delay (Variables|Settings|GetWeapon%20Cooldown%20Duration))
        (goto _label Reset)))))

(event EventTick
  (params (DeltaSeconds :type Float%20%28single-precision%29))
  ;[0 0 0] Pickup Item Code
  ;;[1 1 1] Item Rotation and UpDown Animation
  (Utilities|FlowControl|Gate true
    (:Exit
      (Transformation|AddRelativeRotation (Variables|Default|GetWeaponMesh) (Math|Rotator|MakeRotator 0.0 0.0 (Variables|Settings|GetPickup%20Rotation%20Speed)) false false)
      (Utilities|FlowControl|DoOnce false
        (:Completed
          (Components|Timeline|SetPlayRate (Variables|Default|GetUpDown) (Variables|Settings|GetPickupUpDown%20Speed))
          (bind _height (Timeline|UpDown Play)
            (:Update
              (Transformation|SetRelativeLocation (Variables|Default|GetWeaponMesh) (Math|Vector|MakeVector 0.0 0.0 (* _height (Variables|Settings|GetPickup%20UpDown%20Strength))) false false))))))))

(event EventBeginPlay
  ;[0 0 0] Pickup Item Code
  ;;[1 1 1] Enable Overlap if not Picked Up
  (Utilities|FlowControl|Delay 0.1)
  (if (Variables|Blueprint|GetIsPickedUp?)
    (Variables|Blueprint|SetArmed true)
    (else
      ;;[1 1 1] Pick Up On Overlap
      (CallFunction|Rotate)
      (Utilities|FlowControl|Gate true) ; enters at Open
    )))

(fn ConstructionScript)