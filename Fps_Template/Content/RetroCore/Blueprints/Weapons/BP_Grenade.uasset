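; BP_Grenade is a bouncing projectile grenade that explodes on a timer.
; StartTimer waits out the fuse, triggers BPExplosion for radial damage scaled by the player's damage multiplier, spawns an explosion sprite, hides mesh and trail, then destroys the actor.
; Until detonation, Tick tumbles the mesh at random rotation rates, which are re-rolled on each bounce alongside a bounce sound.
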(event OnProjectileBounce(ProjectileMovement)
  (params (ImpactResult :type Hit%20Result%20Structure%20%28by%20ref%29) (ImpactVelocity :type Vector%20%28by%20ref%29 :default "0, 0, 0"))
  ;[1 1 1] Play Audio on Bounce & Set Random Rotation
  (if (not (Variables|Default|GetExplode?))
    (Audio|PlaySoundatLocation "/Game/RetroCore/Audio/SC_Grenade_Bounce.SC_Grenade_Bounce" (Transformation|GetWorldLocation (Variables|Default|GetSphereCollision)) "0, 0, 0" 1.0 1.0 0.0 0 0 0 0)
    (Variables|Default|SetDelta%20Rotation%20X%20%28Roll%29 (Math|Random|RandomFloatinRange -3.0 3.0))
    (Variables|Default|SetDelta%20Rotation%20Y%20%28Pitch%29 (Math|Random|RandomFloatinRange -3.0 3.0))
    (Variables|Default|SetDelta%20Rotation%20Z%20%28Yaw%29 (Math|Random|RandomFloatinRange -3.0 3.0))))

(event Custom|Start%20Timer
  (Utilities|FlowControl|Delay (Variables|Default|GetExplosion%20Timer))
  (Variables|Default|SetExplode? true)
  (Default|Explode (Variables|Default|GetBP_Explosion) (* (Variables|/Game/RetroCore/Blueprints/Player/BP_FPS_Player.BP_FPS_Player_C|GetDamage%20Multiplier (Variables|Default|GetPlayerUsingThisWeapon)) (Variables|Default|GetBase%20Damage)) (Variables|Default|GetDamage%20Radius))
  (bind _returnvalue (Game|SpawnActorfromClass "/Game/RetroCore/Blueprints/Weapons/BP_Sprite_Explosion.BP_Sprite_Explosion_C" (Math|Transform|MakeTransform (Transformation|GetWorldLocation (Variables|Default|GetSphereCollision)) "0, 0, 0" "1.000000,1.000000,1.000000") "AlwaysSpawn" "MultiplyWithRoot" 0 0))
  (Variables|/Game/RetroCore/Blueprints/Weapons/BP_Sprite_Explosion.BP_Sprite_Explosion_C|SetPlayer%20Reference _returnvalue (Variables|Default|GetPlayerUsingThisWeapon))
  (Components|Activation|Deactivate (Variables|Default|GetNS_Grenade_Trail))
  (Rendering|SetVisibility (Variables|Default|GetSM_Grenade) false false)
  (Utilities|FlowControl|Delay 3.0)
  (Actor|DestroyActor))

(event Custom|Initialize%20Random%20Rotation
  ;[1 1 1] Play Audio on Bounce & Set Random Rotation
  (Variables|Default|SetDelta%20Rotation%20X%20%28Roll%29 (Math|Random|RandomFloatinRange -3.0 3.0))
  (Variables|Default|SetDelta%20Rotation%20Y%20%28Pitch%29 (Math|Random|RandomFloatinRange -3.0 3.0))
  (Variables|Default|SetDelta%20Rotation%20Z%20%28Yaw%29 (Math|Random|RandomFloatinRange -3.0 3.0)))

(event EventTick
  (params (DeltaSeconds :type Float%20%28single-precision%29))
  ;[1 1 1] Add Random Rotation to Mesh
  (if (not (Variables|Default|GetExplode?))
    (Transformation|AddRelativeRotation (Variables|Default|GetSM_Grenade) (Math|Rotator|MakeRotator (Variables|Default|GetDelta%20Rotation%20X%20%28Roll%29) (Variables|Default|GetDelta%20Rotation%20Y%20%28Pitch%29) (Variables|Default|GetDelta%20Rotation%20Z%20%28Yaw%29)) false false)))

(event EventBeginPlay
  (Default|Initialize (Variables|Default|GetBP_Explosion) (Variables|Default|GetRadialForce))
  (CallFunction|InitializeRandomRotation))

(fn ConstructionScript)