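; BP_Sprite_Explosion is a short-lived sprite explosion effect with a flash of light.
; On spawn, a timeline animates the point light's intensity.
; Each tick rotates the flipbook to face the referenced player, offset 90 degrees in yaw, billboard style.
; The actor destroys itself once flipbook playback nearly reaches its end.
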(event EventTick
  (params (DeltaSeconds :type Float%20%28single-precision%29))
  (bind _returnvalue (Transformation|GetActorLocation))
  (bind _flipbook_explosion (Variables|Default|GetFlipbook_Explosion))
  (bind _player_reference (Variables|Default|GetPlayer%20Reference))
  (bind _returnvalue_2 (Transformation|GetActorTransform _player_reference))
  (bind _returnvalue_3 (Math|Rotator|FindLookatRotation _returnvalue (.location _returnvalue_2)))
  (bind (_roll _pitch _yaw) (Math|Rotator|BreakRotator _returnvalue_3))
  (Utilities|IsValid _player_reference
    (:Is%20Valid
      (Transformation|SetWorldRotation (Variables|Default|GetFlipbook_Explosion) (Math|Rotator|MakeRotator _roll _pitch (+ _yaw 9e+01)) false false))
    (:Is%20Not%20Valid
      _))
  (if (Math|Float|NearlyEqual(Float) (Components|Timeline|GetPlaybackPosition _flipbook_explosion) (Class|PaperFlipbookComponent|GetFlipbookLength _flipbook_explosion) 0.05)
    (Actor|DestroyActor)))

(event EventBeginPlay
  (bind _intensity (Timeline|Light%20Animation PlayFromStart)
    (:Update
      (Rendering|Components|Light|SetIntensity (Variables|Default|GetPointLight) (* _intensity 5e+03)))))

(fn ConstructionScript)