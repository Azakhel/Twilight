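; Rocket launcher weapon that serves as both a spinning, bobbing world pickup and the player's armed weapon.
; On overlap, an unpicked launcher hands its class and starting ammo to a player lacking that weapon ID, then destroys itself.
; When armed, Fire spends ammo, spawns BP_Rocket with damage settings, and plays sound and a randomized Niagara muzzle flash.
; A timeline drives light, kickback and rocket reload, while DoOnce plus Delay enforces cooldown.
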(event OnComponentBeginOverlap(Sphere)
  (params (OverlappedComponent :type Primitive%20Component%20Object%20Reference) (OtherActor :type Actor%20Object%20Reference) (OtherComp :type Primitive%20Component%20Object%20Reference) (OtherBodyIndex :type Integer) (bFromSweep :type Boolean) (SweepResult :type Hit%20Result%20Structure%20%28by%20ref%29))
  ;[1 1 1] Pick Up On Overlap
  (Utilities|FlowControl|Gate true
    (:Exit
      (bind _outactors (Actor|GetAllActorsOfClass "/Game/RetroCore/Blueprints/Player/BP_FPS_Player.BP_FPS_Player_C"))
      (for _array_element _outactors
        (if (== _array_element OtherActor)
          (Variables|Blueprint|SetOverlappingPlayer _array_element)
          (Variables|Blueprint|SetFoundPlayer true)
          (if (.ReturnValue (Utilities|Map|Find (Variables|/Game/RetroCore/Blueprints/Player/BP_FPS_Player.BP_FPS_Player_C|GetWeapon%20Inventory%20Class _array_element) (Variables|Settings|GetWeapon%20ID)))
            (Variables|Blueprint|SetIsAlreadyPickedUp? true))))
      (if (Variables|Blueprint|GetFoundPlayer)
        (if (not (Variables|Blueprint|GetIsAlreadyPickedUp?))
          (Default|PickedUpNewWeapon (Variables|Blueprint|GetOverlappingPlayer) (Variables|Settings|GetWeapon%20ID) (Utilities|GetClass self) (Variables|Settings|GetStarting%20Ammunition))
          (Actor|DestroyActor))))))

(event Custom|Rotate
  ;[1 1 1] Item Rotation and UpDown Animation
  (Transformation|SetRelativeScale3D (Variables|Default|GetDefaultSceneRoot) "1.600000,1.600000,1.600000")
  (Utilities|FlowControl|Gate true) ; enters at Open
)

(event Custom|Fire
  ;[1 1 1] Fire Weapon
  (if (Variables|Blueprint|GetArmed)
    (Utilities|FlowControl|Sequence
      (:then_0
        (Utilities|FlowControl|DoOnce false :!label _label
          (:Completed
            (Default|SubtractAmmunition (Variables|Blueprint|GetPlayerUsingThisWeapon))
            (Audio|PlaySoundatLocation "/Game/RetroCore/Audio/SC_Rocket_Launch.SC_Rocket_Launch" (Transformation|GetWorldLocation (Variables|Default|GetPointLight)) "0, 0, 0" 1.0 1.0 0.0 0 0 0 0)
            ;;[1 1 1] Spawn Rocket
            (bind _returnvalue (Game|SpawnActorfromClass "/Game/RetroCore/Blueprints/Weapons/BP_Rocket.BP_Rocket_C" (Transformation|GetWorldTransform (Variables|/Game/RetroCore/Blueprints/Player/BP_FPS_Player.BP_FPS_Player_C|GetLauncherLoc (Variables|Blueprint|GetPlayerUsingThisWeapon))) "AdjustIfPossibleButAlwaysSpawn" "MultiplyWithRoot" 0 0))
            (Variables|/Game/RetroCore/Blueprints/Weapons/BP_Rocket.BP_Rocket_C|SetPlayerUsingThisWeapon _returnvalue (Variables|Blueprint|GetPlayerUsingThisWeapon))
            (Variables|/Game/RetroCore/Blueprints/Weapons/BP_Rocket.BP_Rocket_C|SetBase%20Damage _returnvalue (Variables|Settings|GetBase%20Damage))
            (Variables|/Game/RetroCore/Blueprints/Weapons/BP_Rocket.BP_Rocket_C|SetDamage%20Radius _returnvalue (Variables|Settings|GetRocket%20Damage%20Radius))
            ;;[1 1 1] Muzzle Flash
            (bind _returnvalue_2 (Niagara|SpawnSystemAttached "/Game/RetroCore/Niagara/NS_Muzzle_Flash.NS_Muzzle_Flash" (Variables|Default|GetPointLight) "None" "0, 0, 0" "0, 0, 0" "KeepRelativeOffset" false))
            (bind _returnvalue_3 (Rendering|Material|CreateDynamicMaterialInstance "/Game/RetroCore/Materials/Niagara/M_Muzzle_Flash.M_Muzzle_Flash" "None" "None" :!class /Script/Engine.KismetMaterialLibrary))
            (Rendering|Material|SetTextureParameterValue _returnvalue_3 "Flash Texture" (Utilities|Array|Get(acopy) (Variables|Blueprint|GetMuzzleFlashes) (Math|Random|RandomIntegerinRange 0 7)))
            (Class|NiagaraComponent|SetVariableMaterial _returnvalue_2 "Dynamic Flash" _returnvalue_3)
            (Effects|Components|ParticleSystem|SetColorParameter _returnvalue_2 "Flash Color" "(R=5.000000,G=2.735661,B=0.497275,A=1.000000)")
            ;;[1 1 1] Kickback & Light/Rocket Animation
            (Variables|Blueprint|SetRandom%20Pitch (Math|Random|RandomFloatinRange -1.0 -0.7))
            (Variables|Blueprint|SetRandom%20Yaw (Math|Random|RandomFloatinRange -0.5 0.5))
            (bind (_direction _kickback _light _rocket_reload) (Timeline|Animation PlayFromStart)
              (:Update
                (Rendering|Components|Light|SetIntensity (Variables|Default|GetPointLight) (* _light 3e+03))
                (CallFunction|SetRocketVisiblity)
                (Transformation|SetRelativeLocation (Variables|Default|GetSM_Rocket) (Math|Vector|MakeVector _rocket_reload 0.0 0.0) false false)
                (Transformation|SetRelativeLocation (Variables|Default|GetSM_Rocket_Launcher) (Math|Vector|MakeVector (* _kickback -0.6) 0.0 0.0) false false)
                (Transformation|SetRelativeRotation (Variables|Default|GetSM_Rocket_Launcher) (Math|Rotator|MakeRotator 0.0 (* _kickback (Variables|Blueprint|GetRandom%20Pitch)) (* _kickback (Variables|Blueprint|GetRandom%20Yaw))) false false))))))
      (:then_1
        (Utilities|FlowControl|Delay (Variables|Settings|GetWeapon%20Cooldown%20Duration))
        (goto _label Reset)))))

(event EventTick
  (params (DeltaSeconds :type Float%20%28single-precision%29))
  ;[1 1 1] Item Rotation and UpDown Animation
  (Utilities|FlowControl|Gate true
    (:Exit
      (Transformation|AddRelativeRotation (Variables|Default|GetSM_Rocket_Launcher) (Math|Rotator|MakeRotator 0.0 0.0 (Variables|Settings|GetPickup%20Rotation%20Speed)) false false)
      (Utilities|FlowControl|DoOnce false
        (:Completed
          (Components|Timeline|SetPlayRate (Variables|Default|GetUpDown) (Variables|Settings|GetPickupUpDown%20Speed))
          (bind _height (Timeline|UpDown Play)
            (:Update
              (Transformation|SetRelativeLocation (Variables|Default|GetSM_Rocket_Launcher) (Math|Vector|MakeVector 0.0 0.0 (* _height (Variables|Settings|GetPickup%20UpDown%20Strength))) false false))))))))

(event EventBeginPlay
  ;[1 1 1] Enable Overlap if not Picked Up
  (Utilities|FlowControl|Delay 0.1)
  (if (Variables|Blueprint|GetIsPickedUp?)
    (Variables|Blueprint|SetArmed true)
    (else
      ;[1 1 1] Pick Up On Overlap
      (CallFunction|Rotate)
      (Utilities|FlowControl|Gate true) ; enters at Open
    )))

(fn ConstructionScript)

(fn SetRocketVisiblity
  (bind _weapon_id (Variables|Settings|GetWeapon%20ID))
  (bind _playerusingthisweapon (Variables|Blueprint|GetPlayerUsingThisWeapon))
  (bind _ammunittion (Variables|/Game/RetroCore/Blueprints/Player/BP_FPS_Player.BP_FPS_Player_C|GetAmmunittion _playerusingthisweapon))
  (bind (_value _returnvalue) (Utilities|Map|Find _ammunittion _weapon_id))
  (Rendering|SetVisibility (Variables|Default|GetSM_Rocket) (and (> _value 0) _returnvalue) false))