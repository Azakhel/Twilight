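; BP_Water is a level water volume that affects the first-person player while inside it.
; On BeginPlay it writes its Color into the Water parameter of the MPC_Level material parameter collection.
; Box overlaps with BP_FPS_Player set fall-damage blocking, the in-water flag and a reduced liquid multiplier, then restore defaults on exit.
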(event OnComponentBeginOverlap(Box)
  (params (OverlappedComponent :type Primitive%20Component%20Object%20Reference) (OtherActor :type Actor%20Object%20Reference) (OtherComp :type Primitive%20Component%20Object%20Reference) (OtherBodyIndex :type Integer) (bFromSweep :type Boolean) (SweepResult :type Hit%20Result%20Structure%20%28by%20ref%29))
  ;[1 1 1] Block Fall Damage
  (bind _asbp_fps_player (Utilities|Casting|CastToBP_FPS_Player OtherActor))
  (Variables|/Game/RetroCore/Blueprints/Player/BP_FPS_Player.BP_FPS_Player_C|SetBlock%20Fall%20Damage _asbp_fps_player true)
  (Variables|/Game/RetroCore/Blueprints/Player/BP_FPS_Player.BP_FPS_Player_C|SetIs%20In%20Water _asbp_fps_player true)
  (Variables|/Game/RetroCore/Blueprints/Player/BP_FPS_Player.BP_FPS_Player_C|SetLiquid%20Multiplier _asbp_fps_player 0.7))

(event OnComponentEndOverlap(Box)
  (params (OverlappedComponent :type Primitive%20Component%20Object%20Reference) (OtherActor :type Actor%20Object%20Reference) (OtherComp :type Primitive%20Component%20Object%20Reference) (OtherBodyIndex :type Integer))
  ;[1 1 1] Block Fall Damage
  (bind _asbp_fps_player (Utilities|Casting|CastToBP_FPS_Player OtherActor))
  (Variables|/Game/RetroCore/Blueprints/Player/BP_FPS_Player.BP_FPS_Player_C|SetBlock%20Fall%20Damage _asbp_fps_player false)
  (Variables|/Game/RetroCore/Blueprints/Player/BP_FPS_Player.BP_FPS_Player_C|SetIs%20In%20Water _asbp_fps_player false)
  (Variables|/Game/RetroCore/Blueprints/Player/BP_FPS_Player.BP_FPS_Player_C|SetLiquid%20Multiplier _asbp_fps_player 1.0))

(event EventBeginPlay
  ;[1 1 1] Set Color on Begin Play
  (Rendering|Material|SetVectorParameterValue "/Game/RetroCore/Materials/Level/MPC_Level.MPC_Level" "Water" (Math|Conversions|ToLinearColor(Color) (Variables|Settings|GetColor)) :!class /Script/Engine.KismetMaterialLibrary))

(fn ConstructionScript)