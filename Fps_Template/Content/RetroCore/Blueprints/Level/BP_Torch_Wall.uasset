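; Wall torch actor that shows a flame effect and a moving point light, both tinted by FireColor.
; On BeginPlay it passes a brightened FireColor to the NSTorch effect and the plain color to the light.
; The LightMovement timeline starts at a random position, so torches move out of sync, and drives the light's relative location on each update.
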(event EventBeginPlay
  (bind _fire_color (Variables|Default|GetFire%20Color))
  (Effects|Components|ParticleSystem|SetColorParameter (Variables|Default|GetNS_Torch) "Color" (* _fire_color "(R=50.000000,G=50.000000,B=50.000000,A=1.000000)"))
  (Rendering|Components|Light|SetLightColor (Variables|Default|GetPointLight_Moving) _fire_color true)
  (Components|Timeline|SetPlaybackPosition (Variables|Default|GetLight%20Movement) (Math|Random|RandomFloatinRange 0.0 1.0) false true)
  (bind (_direction _x _y _z) (Timeline|Light%20Movement Play)
    (:Update
      (Transformation|SetRelativeLocation (Variables|Default|GetPointLight_Moving) (Math|Vector|MakeVector _x _y _z) false false))))

(fn ConstructionScript)