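; BP_Toxic_Waste is a toxic liquid hazard volume that slows and periodically damages BP_FPS_Player while it overlaps the box.
; On BeginPlay it writes its color to the ToxicWaste parameter in MPC_Level.
; Box overlaps toggle a Gate and the player's LiquidMultiplier.
; Tick runs through a variable Delay into that Gate, starting at zero for a prompt first hit, then using DurationBetweenDamage until exit resets it.
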(event OnComponentBeginOverlap(Box)
  (params (OverlappedComponent :type Primitive%20Component%20Object%20Reference) (OtherActor :type Actor%20Object%20Reference) (OtherComp :type Primitive%20Component%20Object%20Reference) (OtherBodyIndex :type Integer) (bFromSweep :type Boolean) (SweepResult :type Hit%20Result%20Structure%20%28by%20ref%29))
  ;[1 1 1] Damage Player on Overlap
  (bind _asbp_fps_player (Utilities|Casting|CastToBP_FPS_Player OtherActor))
  (Variables|Blueprint|SetFPS%20Player%20Reference _asbp_fps_player)
  (Variables|/Game/RetroCore/Blueprints/Player/BP_FPS_Player.BP_FPS_Player_C|SetLiquid%20Multiplier _asbp_fps_player 0.6)
  (Utilities|FlowControl|Gate true) ; enters at Open
)

(event OnComponentEndOverlap(Box)
  (params (OverlappedComponent :type Primitive%20Component%20Object%20Reference) (OtherActor :type Actor%20Object%20Reference) (OtherComp :type Primitive%20Component%20Object%20Reference) (OtherBodyIndex :type Integer))
  (bind _fps_player_reference (Variables|Blueprint|GetFPS%20Player%20Reference))
  ;[1 1 1] Damage Player on Overlap
  (if (== OtherActor _fps_player_reference)
    (Variables|Blueprint|SetDelay 0.0)
    (Variables|/Game/RetroCore/Blueprints/Player/BP_FPS_Player.BP_FPS_Player_C|SetLiquid%20Multiplier _fps_player_reference 1.0)
    (Utilities|FlowControl|Gate true) ; enters at Close
  ))

(event EventTick
  (params (DeltaSeconds :type Float%20%28single-precision%29))
  ;[1 1 1] Damage Player on Overlap
  (Utilities|FlowControl|Delay (Variables|Blueprint|GetDelay))
  (Utilities|FlowControl|Gate true
    (:Exit
      (Variables|Blueprint|SetDelay (Variables|Settings|GetDuration%20between%20Damage))
      (Game|Damage|ApplyDamage (Variables|Blueprint|GetFPS%20Player%20Reference) (Variables|Settings|GetBase%20Damage) 0 self))))

(event EventBeginPlay
  ;[1 1 1] Set Color on Begin Play
  (Rendering|Material|SetVectorParameterValue "/Game/RetroCore/Materials/Level/MPC_Level.MPC_Level" "ToxicWaste" (Math|Conversions|ToLinearColor(Color) (Variables|Settings|GetColor)) :!class /Script/Engine.KismetMaterialLibrary))

(fn ConstructionScript)