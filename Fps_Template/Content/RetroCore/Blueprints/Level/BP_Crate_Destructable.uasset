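; A destructible physics crate that breaks apart when its health runs out and drops a random item.
; Impacts play a sound scaled by velocity, throttled by a resettable DoOnce and short delay.
; Damage depletes Health; lethal damage, handled once, hides the main mesh and spawns a random ItemSpawn entry.
; It then reveals pre-built fragment meshes with physics, plays a breaking sound and destroys the actor after a delay.
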(event Game|Damage|EventAnyDamage
  (params (Damage :type Float%20%28single-precision%29) (DamageType :type Damage%20Type%20Object%20Reference) (InstigatedBy :type Controller%20Object%20Reference) (DamageCauser :type Actor%20Object%20Reference))
  (bind _staticmeshcomponent (Variables|Debug|GetStaticMeshComponent))
  ;[1 1 1] Destruction on Event Damage
  (if (> (- (Variables|Default|GetHealth) Damage) 0.0)
    (Variables|Default|SetHealth (- (Variables|Default|GetHealth) Damage))
    (else
      (Utilities|FlowControl|DoOnce false
        (:Completed
          (Development|SetHiddeninGame _staticmeshcomponent true false)
          (Physics|SetSimulatePhysics _staticmeshcomponent false)
          (Collision|SetCollisionEnabled _staticmeshcomponent "NoCollision")
          (Game|SpawnActorfromClass (Utilities|Array|Get(acopy) (Variables|Default|GetItem%20Spawn) (Math|Random|RandomIntegerinRange 0 7)) (Transformation|GetActorTransform) "AlwaysSpawn" "MultiplyWithRoot" 0 0)
          (Development|SetHiddeninGame (Variables|Default|GetSM_Crate_Fragment_05) false false)
          (Physics|SetSimulatePhysics (Variables|Default|GetSM_Crate_Fragment_05) true)
          (Audio|PlaySoundatLocation "/Game/RetroCore/Audio/SC_Crate_Braking.SC_Crate_Braking" (Transformation|GetActorLocation) "0, 0, 0" 1.0 1.0 0.0 0 0 0 0)
          (Utilities|FlowControl|Delay 5.0)
          (Actor|DestroyActor))))))

(event Collision|EventHit
  (params (MyComp :type Primitive%20Component%20Object%20Reference) (Other :type Actor%20Object%20Reference) (OtherComp :type Primitive%20Component%20Object%20Reference) (bSelfMoved :type Boolean) (HitLocation :type Vector :default "0, 0, 0") (HitNormal :type Vector :default "0, 0, 0") (NormalImpulse :type Vector :default "0, 0, 0") (Hit :type Hit%20Result%20Structure%20%28by%20ref%29))
  ;[1 1 1] Play Audio on Event Hit
  (Utilities|FlowControl|DoOnce false :!label _label
    (:Completed
      (Audio|PlaySoundatLocation "/Game/RetroCore/Audio/SC_Crate.SC_Crate" HitLocation "0, 0, 0" (Math|Float|Clamp(Float) (/ (Math|Vector|VectorLength (Transformation|GetVelocity)) 1.2e+03) 0.0 0.7) 1.0 0.0 0 0 0 0)
      (Utilities|FlowControl|Delay 0.5)
      (goto _label Reset))))

(fn ConstructionScript)